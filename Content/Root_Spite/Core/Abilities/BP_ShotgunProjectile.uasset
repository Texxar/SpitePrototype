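; BP_ShotgunProjectile is a short-range shotgun projectile that damages BP_Enemy actors it overlaps.
; Tick moves it along its forward vector in X and Y by ProjectileSpeed per frame, without sweep or delta-time scaling, so speed depends on frame rate.
; A static mesh overlap with an enemy applies fixed damage and destroys the projectile; otherwise a brief BeginPlay delay destroys it, limiting range.
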(event OnComponentBeginOverlap(StaticMesh)
  (params (OverlappedComponent :type Primitive%20Component%20Object%20Reference) (OtherActor :type Actor%20Object%20Reference) (OtherComp :type Primitive%20Component%20Object%20Reference) (OtherBodyIndex :type Integer) (bFromSweep :type Boolean) (SweepResult :type Hit%20Result%20Structure%20%28by%20ref%29))
  (bind _asbp_enemy (Utilities|Casting|CastToBP_Enemy OtherActor))
  (Game|Damage|ApplyDamage _asbp_enemy 5.0 0 0)
  (Actor|DestroyActor))

(event EventTick
  (params (DeltaSeconds :type Float%20%28single-precision%29))
  (bind _projectilespeed (Variables|Default|GetProjectileSpeed))
  (Transformation|SetActorLocation (+ (Transformation|GetActorLocation) (* (Math|Vector|GetForwardVector (Transformation|GetActorRotation)) (Math|Vector|MakeVector _projectilespeed _projectilespeed 0.0))) false false))

(event EventBeginPlay
  (Utilities|FlowControl|Delay 0.4)
  (Actor|DestroyActor))

(fn ConstructionScript)