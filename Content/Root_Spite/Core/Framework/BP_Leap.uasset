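; BP_Leap is a Blueprint that makes the player character leap from its current position to a given landing location.
; On BeginPlay it records the start location and turns the character toward the landing point, ignoring height.
; A timeline then sets the location each update, blending start to landing with a Movement track and adding a vertical offset from a Height track to shape the jump.
; The movement does not sweep for collision.
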(event EventBeginPlay
  (Variables|Default|SetStartLocation (Transformation|GetActorLocation (Variables|Default|GetPlayerCharacterRef)))
  (Transformation|SetActorRotation (Variables|Default|GetPlayerCharacterRef) (Math|Rotator|FindLookatRotation (* (Variables|Default|GetStartLocation) "1.000000,1.000000, 0") (* (Variables|Default|GetLandLocation) "1.000000,1.000000, 0")))
  (bind (_direction _movement _height) (Timeline|Timeline_0 PlayFromStart)
    (:Update
      (Transformation|SetActorLocation (Variables|Default|GetPlayerCharacterRef) (+ (Math|Vector|Lerp(Vector) (Variables|Default|GetStartLocation) (Variables|Default|GetLandLocation) _movement) (Math|Vector|Lerp(Vector) "0, 0, 0" "0, 0,500.000000" _height)) false false))))

(fn ConstructionScript)