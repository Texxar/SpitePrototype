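; BP_ExpOrb is an experience pickup that scatters from its spawn point, then homes in on the player.
; On BeginPlay a timeline arcs it to a random navigable point nearby, using separate travel and height tracks.
; After a short delay a gate opens, letting Tick interpolate it toward player character 0.
; Overlapping a Core_SpiteCharacter grants fixed experience, plays a sound and destroys the orb.
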(event OnComponentBeginOverlap(PickupCollider)
  (params (OverlappedComponent :type Primitive%20Component%20Object%20Reference) (OtherActor :type Actor%20Object%20Reference) (OtherComp :type Primitive%20Component%20Object%20Reference) (OtherBodyIndex :type Integer) (bFromSweep :type Boolean) (SweepResult :type Hit%20Result%20Structure%20%28by%20ref%29))
  (bind _ascore_spite_character (Utilities|Casting|CastToCore_SpiteCharacter OtherActor))
  (Default|AddExp _ascore_spite_character 5.0)
  (Audio|PlaySoundatLocation "/Game/Root_Spite/Core/Framework/Rost_007_sd.Rost_007_sd" (Transformation|GetActorLocation) "0, 0, 0" 1.0 1.0 0.0 0 0 0)
  (Actor|DestroyActor))

(event EventBeginPlay
  (bind _output_get (Variables|Default|SetStartLocation (Transformation|GetActorLocation)))
  (bind _randomlocation (Class|NavigationSystemV1|GetRandomLocationinNavigableRadius _output_get 5e+02 0 0))
  (Variables|Default|SetEndLocation _randomlocation)
  (bind (_direction _tolocation _height) (Timeline|Timeline_0 PlayFromStart)
    (:Update
      (Transformation|SetActorLocation (+ (Math|Vector|Lerp(Vector) (Variables|Default|GetStartLocation) (Variables|Default|GetEndLocation) _tolocation) (Math|Vector|MakeVector 0.0 0.0 (* _height 3e+02))) false false))
    (:Finished
      (Utilities|FlowControl|Delay 0.3)
      (Utilities|FlowControl|Gate true) ; enters at Open
    )))

(event EventTick
  (params (DeltaSeconds :type Float%20%28single-precision%29))
  (Utilities|FlowControl|Gate true
    (:Exit
      (Transformation|SetActorLocation (Math|Interpolation|VInterpTo (Transformation|GetActorLocation) (Transformation|GetActorLocation (Game|GetPlayerCharacter 0)) DeltaSeconds 2.0) false false))))

(fn ConstructionScript)