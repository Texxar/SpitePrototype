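; BP_Slam is a short-lived player ability actor that delivers a slam attack, damaging enemies it touches.
; On BeginPlay it offsets and stretches the Cone to match the LightAttackData range.
; A sped-up timeline rotates and grows ConeStart from zero to full scale, then destroys the actor.
; Box overlaps with BP_Enemy actors apply the LightAttackData damage.
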(event OnComponentBeginOverlap(Box)
  (params (OverlappedComponent :type Primitive%20Component%20Object%20Reference) (OtherActor :type Actor%20Object%20Reference) (OtherComp :type Primitive%20Component%20Object%20Reference) (OtherBodyIndex :type Integer) (bFromSweep :type Boolean) (SweepResult :type Hit%20Result%20Structure%20%28by%20ref%29))
  (bind _asbp_enemy (Utilities|Casting|CastToBP_Enemy OtherActor))
  (Game|Damage|ApplyDamage _asbp_enemy (.damage (Variables|Default|GetLightAttackData)) 0 0))

(event EventBeginPlay
  (bind _lightattackdata (Variables|Default|GetLightAttackData))
  (bind _cone (Variables|Default|GetCone))
  (Transformation|SetRelativeLocation _cone (Math|Vector|MakeVector (/ (.range _lightattackdata) 2.0) 0.0 0.0) false false)
  (Transformation|SetRelativeScale3D _cone (Math|Vector|MakeVector 1.0 1.0 (/ (.range _lightattackdata) 1e+02)))
  (Components|Timeline|SetPlayRate (Variables|Default|GetTimeline_0) 1.5)
  (bind (_direction _location _rotation _scale) (Timeline|Timeline_0 PlayFromStart)
    (:Update
      (Transformation|SetRelativeTransform (Variables|Default|GetConeStart) (Math|Transform|MakeTransform "0, 0, 0" (Math|Rotator|Lerp(Rotator) "90.000000, 0, 0" "0, 0, 0" _rotation true) (Math|Vector|Lerp(Vector) "0, 0, 0" "1.000000,1.000000,1.000000" _scale)) false false))
    (:Finished
      (Actor|DestroyActor))))

(fn ConstructionScript)