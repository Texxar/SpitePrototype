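; BP_Leap is a player ability actor that makes the Spite character leap to the cursor location and slam down.
; On BeginPlay it records the character's position and the player cursor's position, then turns the character to face the target on the horizontal plane.
; A timeline lerps the character along that path with an added height curve for the arc, without sweeping.
; When it finishes, it spawns BP_Groundpound at the landing point and destroys itself.
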(event EventBeginPlay
  (bind _output_get (Variables|Default|SetPlayerCharacterRef (.AsCore%20Spite%20Character (Utilities|Casting|CastToCore_SpiteCharacter (Game|GetPlayerCharacter 0)))))
  (Variables|Default|SetStartLocation (Transformation|GetActorLocation _output_get))
  (bind _outactors (Actor|GetAllActorsOfClass "/Game/Root_Spite/Core/Player/Core_SpitePlayerCursor.Core_SpitePlayerCursor_C"))
  (Variables|Default|SetLandLocation (Transformation|GetActorLocation (Utilities|Array|Get(acopy) _outactors)))
  (Transformation|SetActorRotation (Variables|Default|GetPlayerCharacterRef) (Math|Rotator|FindLookatRotation (* (Variables|Default|GetStartLocation) "1.000000,1.000000, 0") (* (Variables|Default|GetLandLocation) "1.000000,1.000000, 0")))
  (bind (_direction _movement _height) (Timeline|Timeline_0 PlayFromStart)
    (:Update
      (Transformation|SetActorLocation (Variables|Default|GetPlayerCharacterRef) (+ (Math|Vector|Lerp(Vector) (Variables|Default|GetStartLocation) (Variables|Default|GetLandLocation) _movement) (Math|Vector|Lerp(Vector) "0, 0, 0" "0, 0,500.000000" _height)) false false))
    (:Finished
      (Game|SpawnActorfromClass "/Game/Root_Spite/Core/Player/Abilities/BP_Groundpound.BP_Groundpound_C" (Math|Transform|MakeTransform (Variables|Default|GetLandLocation) "0, 0, 0" "1,1,1") "Undefined" 0 0)
      (Actor|DestroyActor))))

(fn ConstructionScript)