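; BP_Shotgun is a player ability actor that fires a fan of shotgun projectiles toward the cursor.
; On BeginPlay it takes its own location as the origin and aims at the first Core_SpitePlayerCursor actor found in the level.
; It spawns BP_ShotgunProjectile actors in a loop, stepping yaw by ArcDegree divided by NumberOfProjectiles, starting half the arc to one side of the aim direction.
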(event EventBeginPlay
  (Variables|Default|SetPlayerLocation (Transformation|GetActorLocation))
  (bind _outactors (Actor|GetAllActorsOfClass "/Game/Root_Spite/Core/Player/Core_SpitePlayerCursor.Core_SpitePlayerCursor_C"))
  (Variables|Default|SetMouseLocation (Transformation|GetActorLocation (Utilities|Array|Get(acopy) _outactors)))
  (Variables|Default|SetDegreesBetweenProjectiles (/ (Variables|Default|GetArcDegree) (Math|Conversions|ToFloat(Integer) (Variables|Default|GetNumberOfProjectiles))))
  (for _index (range 0 (Variables|Default|GetNumberOfProjectiles))
    (Game|SpawnActorfromClass "/Game/Root_Spite/Core/Player/Abilities/BP_ShotgunProjectile.BP_ShotgunProjectile_C" (Math|Transform|MakeTransform (Transformation|GetActorLocation) (Math|Rotator|CombineRotators (Math|Rotator|FindLookatRotation (Variables|Default|GetPlayerLocation) (Variables|Default|GetMouseLocation)) (Math|Rotator|MakeRotator 0.0 0.0 (+ (* _index (Variables|Default|GetDegreesBetweenProjectiles)) (* (/ (Variables|Default|GetArcDegree) 2.0) -1.0)))) "1,1,1") "Undefined" 0 0)))

(fn ConstructionScript)