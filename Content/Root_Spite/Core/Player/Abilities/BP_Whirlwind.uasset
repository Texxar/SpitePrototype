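; BP_Whirlwind is a player ability actor that damages enemies in an expanding area and heals the player for each hit.
; On BeginPlay it deducts the mana cost, then a timeline scales a flattened sphere from zero out to the configured radius.
; Each BP_Enemy overlap deals damage and heals the player through negative ApplyDamage, with all tuning read from WhirlwindData.
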(event OnComponentBeginOverlap(Sphere)
  (params (OverlappedComponent :type Primitive%20Component%20Object%20Reference) (OtherActor :type Actor%20Object%20Reference) (OtherComp :type Primitive%20Component%20Object%20Reference) (OtherBodyIndex :type Integer) (bFromSweep :type Boolean) (SweepResult :type Hit%20Result%20Structure%20%28by%20ref%29))
  (bind _whirlwinddata (Variables|Default|GetWhirlwindData))
  (bind _asbp_enemy (Utilities|Casting|CastToBP_Enemy OtherActor))
  (Game|Damage|ApplyDamage _asbp_enemy (.damage _whirlwinddata) 0 0)
  (Game|Damage|ApplyDamage (Variables|Default|GetPlayerCharacterRef) (* (.hpgainperenemyhit _whirlwinddata) -1.0) 0 0))

(event EventBeginPlay
  (bind _whirlwinddata (Variables|Default|GetWhirlwindData))
  (bind _returnvalue (/ (.radius _whirlwinddata) 5e+01))
  (Default|OnUpdateMana (Variables|Default|GetPlayerCharacterRef) (* (.manacost _whirlwinddata) -1.0))
  (bind _scale (Timeline|Timeline_0 PlayFromStart)
    (:Update
      (Transformation|SetWorldScale3D (Variables|Default|GetSphere) (Math|Vector|Lerp(Vector) "0, 0, 0" (Math|Vector|MakeVector _returnvalue _returnvalue 0.1) _scale)))))

(fn ConstructionScript)