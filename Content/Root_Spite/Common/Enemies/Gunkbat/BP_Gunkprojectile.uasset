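; BP_Gunkprojectile is the lobbed projectile in the Gunkbat enemy's folder, leaving a gunk pool where it lands.
; On BeginPlay it stores its start location and plays a timeline that lerps it toward HitLocation, adding a curve-driven vertical offset to form an arc without physics or sweep.
; When the timeline finishes, it spawns BP_Gunkpool at HitLocation and destroys itself.
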(event EventBeginPlay
  (Variables|Default|SetStartLocation (Transformation|GetActorLocation))
  (bind (_direction _alpha _curve) (Timeline|Timeline_0 PlayFromStart)
    (:Update
      (Transformation|SetActorLocation (+ (Math|Vector|Lerp(Vector) (Variables|Default|GetStartLocation) (Variables|Default|GetHitLocation) _alpha) (Math|Vector|Lerp(Vector) "0, 0, 0" "0, 0,500.000000" _curve)) false false))
    (:Finished
      (Game|SpawnActorfromClass "/Game/Root_Spite/Common/Enemies/Gunkbat/BP_Gunkpool.BP_Gunkpool_C" (Math|Transform|MakeTransform (Variables|Default|GetHitLocation) "0, 0, 0" "1,1,1") "Undefined" 0 0)
      (Actor|DestroyActor))))

(fn ConstructionScript)