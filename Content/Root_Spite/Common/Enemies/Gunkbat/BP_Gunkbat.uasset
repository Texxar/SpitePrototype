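; BP_Gunkbat is a ranged enemy that attacks the player from a distance and flees when approached.
; Overlaps on two triggers, AggroTrigger and CloseTrigger, switch its state between Idle, Attack and Flee.
; Tick halts movement and fires gunk projectiles at the player on a cooldown, or moves to a rotated-vector escape point, while setting yaw along the player-to-bat direction.
; The AggroRange radius setter is unconnected.
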(event OnComponentBeginOverlap(AggroTrigger)
  (params (OverlappedComponent :type Primitive%20Component%20Object%20Reference) (OtherActor :type Actor%20Object%20Reference) (OtherComp :type Primitive%20Component%20Object%20Reference) (OtherBodyIndex :type Integer) (bFromSweep :type Boolean) (SweepResult :type Hit%20Result%20Structure%20%28by%20ref%29))
  (Utilities|Casting|CastToCore_SpiteCharacter OtherActor)
  (Variables|Default|SetEnemyState_0 "NewEnumerator1"))

(event OnComponentEndOverlap(AggroTrigger)
  (params (OverlappedComponent :type Primitive%20Component%20Object%20Reference) (OtherActor :type Actor%20Object%20Reference) (OtherComp :type Primitive%20Component%20Object%20Reference) (OtherBodyIndex :type Integer))
  (Utilities|Casting|CastToCore_SpiteCharacter OtherActor)
  (Variables|Default|SetEnemyState_0 "NewEnumerator0"))

(event OnComponentEndOverlap(CloseTrigger)
  (params (OverlappedComponent :type Primitive%20Component%20Object%20Reference) (OtherActor :type Actor%20Object%20Reference) (OtherComp :type Primitive%20Component%20Object%20Reference) (OtherBodyIndex :type Integer))
  (Utilities|Casting|CastToCore_SpiteCharacter OtherActor)
  (Variables|Default|SetEnemyState_0 "NewEnumerator1"))

(event OnComponentBeginOverlap(CloseTrigger)
  (params (OverlappedComponent :type Primitive%20Component%20Object%20Reference) (OtherActor :type Actor%20Object%20Reference) (OtherComp :type Primitive%20Component%20Object%20Reference) (OtherBodyIndex :type Integer) (bFromSweep :type Boolean) (SweepResult :type Hit%20Result%20Structure%20%28by%20ref%29))
  (Utilities|Casting|CastToCore_SpiteCharacter OtherActor)
  (Variables|Default|SetEnemyState_0 "NewEnumerator2"))

(event EventBeginPlay
  (|CallParentFunction))

(event EventTick
  (params (DeltaSeconds :type Float%20%28single-precision%29))
  (bind _returnvalue (Transformation|GetActorLocation))
  (bind _runawaylocation (Variables|Default|GetRunAwayLocation))
  (Utilities|FlowControl|Sequence
    (:then_0
      (switch Utilities|FlowControl|Switch|SwitchonE_EnemyStates (Variables|Default|GetEnemyState_0)
        (:NewEnumerator1
          (Class|NavMovementComponent|StopActiveMovement (Variables|Character|GetCharacterMovement))
          (Utilities|FlowControl|DoOnce false :!label _label
            (:Completed
              (Game|SpawnActorfromClass "/Game/Root_Spite/Common/Enemies/Gunkbat/BP_Gunkprojectile.BP_Gunkprojectile_C" (Transformation|GetActorTransform) "Undefined" 0 (Transformation|GetActorLocation (Game|GetPlayerCharacter 0)) 0)
              (Utilities|FlowControl|Delay 1.0)
              (goto _label Reset))))
        (:NewEnumerator2
          (Transformation|SetWorldLocation _runawaylocation (+ (Math|Vector|RotateVector (- (Transformation|GetActorLocation (Game|GetPlayerCharacter 0)) _returnvalue) "0,180.000000, 0") _returnvalue) false false)
          (AI|Navigation|SimpleMovetoLocation (Pawn|GetController) (Transformation|GetWorldLocation _runawaylocation)))))
    (:then_1
      (Transformation|SetActorRotation (Math|Rotator|MakeRotator 0.0 0.0 (.yaw (Math|Rotator|FindLookatRotation (Transformation|GetActorLocation (Game|GetPlayerCharacter 0)) (Transformation|GetActorLocation))))))))

(fn ConstructionScript
  (|CallParentFunction))