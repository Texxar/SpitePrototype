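; Ribleech enemy that chases and attacks Spite characters, driven by a state switch on Tick.
; Aggro and attack trigger overlaps set Idle, Chase or Attack; Bloodletting actors also trigger Chase, though movement always follows the player.
; Attack snapshots the target's location, briefly waits, then spawns a LeechAttack behind a cooldown-reset DoOnce.
; Flee, never set here, moves toward the stored target, and the aggro-radius setter is unconnected.
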(event OnComponentBeginOverlap(AggroTrigger)
  (params (OverlappedComponent :type Primitive%20Component%20Object%20Reference) (OtherActor :type Actor%20Object%20Reference) (OtherComp :type Primitive%20Component%20Object%20Reference) (OtherBodyIndex :type Integer) (bFromSweep :type Boolean) (SweepResult :type Hit%20Result%20Structure%20%28by%20ref%29))
  (bind _asbp_bloodletting (Utilities|Casting|CastToBP_Bloodletting OtherActor)
    (:then
      (Variables|Default|SetChaseTarget _asbp_bloodletting))
    (:CastFailed
      (bind _ascore_spite_character (Utilities|Casting|CastToCore_SpiteCharacter OtherActor))
      (Variables|Default|SetChaseTarget _ascore_spite_character)))
  (Variables|Default|SetState "NewEnumerator3"))

(event OnComponentBeginOverlap(AttackTrigger)
  (params (OverlappedComponent :type Primitive%20Component%20Object%20Reference) (OtherActor :type Actor%20Object%20Reference) (OtherComp :type Primitive%20Component%20Object%20Reference) (OtherBodyIndex :type Integer) (bFromSweep :type Boolean) (SweepResult :type Hit%20Result%20Structure%20%28by%20ref%29))
  (Utilities|Casting|CastToCore_SpiteCharacter OtherActor)
  (Variables|Default|SetState "NewEnumerator1"))

(event OnComponentEndOverlap(AttackTrigger)
  (params (OverlappedComponent :type Primitive%20Component%20Object%20Reference) (OtherActor :type Actor%20Object%20Reference) (OtherComp :type Primitive%20Component%20Object%20Reference) (OtherBodyIndex :type Integer))
  (Utilities|Casting|CastToCore_SpiteCharacter OtherActor)
  (Variables|Default|SetState "NewEnumerator3"))

(event OnComponentEndOverlap(AggroTrigger)
  (params (OverlappedComponent :type Primitive%20Component%20Object%20Reference) (OtherActor :type Actor%20Object%20Reference) (OtherComp :type Primitive%20Component%20Object%20Reference) (OtherBodyIndex :type Integer))
  (Utilities|Casting|CastToCore_SpiteCharacter OtherActor)
  (Variables|Default|SetState "NewEnumerator0"))

(event Custom|OnSetMoveToLocation
  (params (Location :type Vector))
  (AI|Navigation|SimpleMovetoLocation (Pawn|GetController) Location))

(event EventBeginPlay
  (|CallParentFunction))

(event Collision|EventActorBeginOverlap
  (params (OtherActor :type Actor%20Object%20Reference)))

(event EventTick
  (params (DeltaSeconds :type Float%20%28single-precision%29))
  (switch Utilities|FlowControl|Switch|SwitchonE_EnemyStates (Variables|Default|GetState)
    (:NewEnumerator3
      (AI|Navigation|SimpleMovetoActor (Pawn|GetController) (Game|GetPlayerCharacter 0)))
    (:NewEnumerator1
      (Utilities|FlowControl|DoOnce false :!label _label
        (:Completed
          (Variables|Default|SetAttackLocation (Transformation|GetActorLocation (Variables|Default|GetChaseTarget)))
          (Utilities|FlowControl|Delay 0.2)
          (Game|SpawnActorfromClass "/Game/Root_Spite/Common/Enemies/BP_LeechAttack.BP_LeechAttack_C" (Math|Transform|MakeTransform (Transformation|GetActorLocation) "0, 0, 0" "1,1,1") "Undefined" 0 (Variables|Default|GetAttackLocation) 0)
          (Utilities|FlowControl|Delay 1.0)
          (goto _label Reset))))
    (:NewEnumerator2
      (AI|Navigation|SimpleMovetoActor (Pawn|GetController) (Variables|Default|GetChaseTarget)))))

(fn ConstructionScript
  (|CallParentFunction))