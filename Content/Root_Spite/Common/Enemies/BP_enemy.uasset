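; BP_enemy is an enemy actor that takes damage and drops experience orbs when it dies.
; On begin play it sets itself as the owner of the HealthBar widget held by its widget component.
; Any damage is subtracted from CurrentHealth, and at zero or below it spawns a batch of BP_ExpOrb actors at its location, then destroys itself.
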(event EventBeginPlay
  (bind _ashealth_bar (Utilities|Casting|CastToHealthBar (UserInterface|GetUserWidgetObject (Variables|Default|GetHealthBar))))
  (Variables|/Game/Root_Spite/Core/UI/HealthBar.HealthBar_C|SetOwner _ashealth_bar self))

(event Game|Damage|EventAnyDamage
  (params (Damage :type Float%20%28single-precision%29) (DamageType :type Damage%20Type%20Object%20Reference) (InstigatedBy :type Controller%20Object%20Reference) (DamageCauser :type Actor%20Object%20Reference))
  (bind _output_get (Variables|Default|SetCurrentHealth (- (Variables|Default|GetCurrentHealth) Damage)))
  (if (<= _output_get 0.0)
    (for _index (range 0 15)
      (Game|SpawnActorfromClass "/Game/Root_Spite/Core/Framework/BP_ExpOrb.BP_ExpOrb_C" (Math|Transform|MakeTransform (Transformation|GetActorLocation) "0, 0, 0" "1,1,1") "Undefined" 0 0))
    (Actor|DestroyActor)))

(fn ConstructionScript)