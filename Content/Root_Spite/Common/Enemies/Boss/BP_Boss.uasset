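; Boss enemy that faces the player, sets a Chase/Attack blackboard state from trigger overlaps, and drops XP orbs on death.
; OnAttack alternates a spawned attack and mouth sonic wave on a one-second cooldown.
; Damage advances health-threshold phases; Ribleeches touching the mouth are timeline-pulled in, counted and destroyed.
; The per-phase logic (chase, jump, Ribleech suction, gunk blast scaled by enemies eaten) is unwired and never runs.
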(event OnComponentBeginOverlap(AggroTrigger)
  (params (OverlappedComponent :type Primitive%20Component%20Object%20Reference) (OtherActor :type Actor%20Object%20Reference) (OtherComp :type Primitive%20Component%20Object%20Reference) (OtherBodyIndex :type Integer) (bFromSweep :type Boolean) (SweepResult :type Hit%20Result%20Structure%20%28by%20ref%29))
  (Utilities|Casting|CastToCore_SpiteCharacter OtherActor)
  (bind _output_get (Variables|Default|SetState "NewEnumerator3"))
  (AI|Components|Blackboard|SetValueasEnum (AI|GetBlackboard 0) (Variables|Default|GetBB_StateName) _output_get))

(event OnComponentBeginOverlap(CloseTrigger)
  (params (OverlappedComponent :type Primitive%20Component%20Object%20Reference) (OtherActor :type Actor%20Object%20Reference) (OtherComp :type Primitive%20Component%20Object%20Reference) (OtherBodyIndex :type Integer) (bFromSweep :type Boolean) (SweepResult :type Hit%20Result%20Structure%20%28by%20ref%29))
  (Utilities|Casting|CastToCore_SpiteCharacter OtherActor)
  (bind _output_get (Variables|Default|SetState "NewEnumerator1"))
  (AI|Components|Blackboard|SetValueasEnum (AI|GetBlackboard 0) (Variables|Default|GetBB_StateName) _output_get))

(event OnComponentEndOverlap(CloseTrigger)
  (params (OverlappedComponent :type Primitive%20Component%20Object%20Reference) (OtherActor :type Actor%20Object%20Reference) (OtherComp :type Primitive%20Component%20Object%20Reference) (OtherBodyIndex :type Integer))
  (Utilities|Casting|CastToCore_SpiteCharacter OtherActor)
  (bind _output_get (Variables|Default|SetState "NewEnumerator3"))
  (AI|Components|Blackboard|SetValueasEnum (AI|GetBlackboard 0) (Variables|Default|GetBB_StateName) _output_get))

(event OnComponentBeginOverlap(MouthCollision)
  (params (OverlappedComponent :type Primitive%20Component%20Object%20Reference) (OtherActor :type Actor%20Object%20Reference) (OtherComp :type Primitive%20Component%20Object%20Reference) (OtherBodyIndex :type Integer) (bFromSweep :type Boolean) (SweepResult :type Hit%20Result%20Structure%20%28by%20ref%29))
  (bind _asbp_ribleech (Utilities|Casting|CastToBP_Ribleech OtherActor))
  (Variables|Default|SetbEatEnemy true)
  (Variables|Default|SetMonchStartLocation (Transformation|GetActorLocation _asbp_ribleech))
  (Collision|SetActorEnableCollision _asbp_ribleech false)
  (Components|Movement|StopMovementImmediately (Variables|/Script/Engine.Character|GetCharacterMovement _asbp_ribleech))
  (bind _newtrack_0 (Timeline|Timeline_0 PlayFromStart)
    (:Update
      (Transformation|SetActorLocation _asbp_ribleech (Math|Vector|Lerp(Vector) (Variables|Default|GetMonchStartLocation) (Transformation|GetSocketLocation (Variables|Character|GetMesh) "Mouth") _newtrack_0) false false))
    (:Finished
      (Math|Integer|IncrementInt (Variables|Default|GetEnemies%20Eaten)
        (:%20%20
          (Variables|Default|SetbEatEnemy false)
          (Utilities|IsValid _asbp_ribleech
            (:Is%20Valid
              (Actor|DestroyActor _asbp_ribleech))))))))

(event Custom|OnAttack
  ;[1 1 1] Phase 1 attack cycle
  (Utilities|FlowControl|DoOnce false :!label _label
    (:Completed
      (bind _isa (Utilities|FlowControl|FlipFlop)
        (:A
          (Game|SpawnActorfromClass "/Game/Root_Spite/Common/Enemies/Boss/Attacks/BP_BossAttack.BP_BossAttack_C" (Math|Transform|MakeTransform (Transformation|GetActorLocation) (Transformation|GetActorRotation) "1,1,1") "Undefined" 0 0))
        (:B
          (Game|SpawnActorfromClass "/Game/Root_Spite/Common/Enemies/Boss/Attacks/BP_BossSonicWave.BP_BossSonicWave_C" (Math|Transform|MakeTransform (Transformation|GetSocketLocation (Variables|Character|GetMesh) "Mouth") (Transformation|GetActorRotation) "1,1,1") "Undefined" 0 0)))
      (Variables|Default|SetAttackSwitcher _isa)
      (Utilities|FlowControl|Delay 1.0)
      (goto _label Reset))))

(event EventBeginPlay
  (bind _healthbar (Variables|Default|GetHealthBar))
  (bind _returnvalue (UserInterface|GetUserWidgetObject _healthbar))
  (|CallParentFunction)
  (bind _ascore_spite_character (Utilities|Casting|CastToCore_SpiteCharacter (Game|Player|GetPlayerPawn 0)))
  (Variables|Default|SetPlayerCharacterRef _ascore_spite_character)
  (UserInterface|Viewport|AddtoViewport _returnvalue 0)
  (Development|SetHiddeninGame (Variables|Default|GetHealthBar) true false)
  (Variables|/Game/Root_Spite/Core/UI/BossHealthBar.BossHealthBar_C|SetOwner (.AsBoss%20Health%20Bar (Utilities|Casting|CastToBossHealthBar _returnvalue)) self)
  (CallFunction|SetHealth 1e+03))

(event Game|Damage|EventAnyDamage
  (params (Damage :type Float%20%28single-precision%29) (DamageType :type Damage%20Type%20Object%20Reference) (InstigatedBy :type Controller%20Object%20Reference) (DamageCauser :type Actor%20Object%20Reference))
  ;[1 1 1] Take damage
  (bind _output_get (Variables|Default|SetCurrentHealth (- (Variables|Default|GetCurrentHealth) Damage)))
  ;[1 1 1] Die
  (if (<= _output_get 0.0)
    (Utilities|FlowControl|DoOnce false
      (:Completed
        (Variables|Default|SetbIsDead true)
        (for _index (range 0 (Variables|Default|GetExpOnKill))
          (Game|SpawnActorfromClass "/Game/Root_Spite/Core/Framework/BP_ExpOrb.BP_ExpOrb_C" (Math|Transform|MakeTransform (Transformation|GetActorLocation) "0, 0, 0" "1,1,1") "Undefined" 0 0))))
    (else
      ;[1 1 1] Phase 3
      (if (<= _output_get (Variables|Default|GetPhase3Threshold))
        (Variables|Default|SetPhase "NewEnumerator2")
        (else
          ;[1 1 1] Phase 2
          (if (<= _output_get (Variables|Default|GetPhase2Threshold))
            (Variables|Default|SetPhase "NewEnumerator1")
            (Variables|Default|SetState "NewEnumerator0")))))))

(event EventTick
  (params (DeltaSeconds :type Float%20%28single-precision%29))
  (if (not (Variables|Default|GetbIsDead))
    (Utilities|FlowControl|Sequence
      (:then_0
        ;[1 1 1] Rotate
        (Transformation|SetActorRotation (Math|Rotator|MakeRotator 0.0 0.0 (.yaw (Math|Interpolation|RInterpTo (Transformation|GetActorRotation) (Math|Rotator|FindLookatRotation (Transformation|GetActorLocation) (Transformation|GetActorLocation (Variables|Default|GetPlayerCharacterRef))) DeltaSeconds 5.0))))))))

(fn ConstructionScript
  (|CallParentFunction))