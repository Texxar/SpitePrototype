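; Boss attack actor that fires a gunk blast as a line of BP_Gunkprojectile spawns.
; On BeginPlay it loops over NumberOfProjectiles, spawning each projectile at its own location with a different HitLocation.
; Hit locations step along Direction at intervals of MaxDistance divided by the projectile count, starting at zero.
; HitLocation is computed without adding the actor's location.
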(event EventBeginPlay
  (for _index (range 0 (+ (Variables|Default|GetNumberOfProjectiles) 1))
    (Game|SpawnActorfromClass "/Game/Root_Spite/Common/Enemies/BP_Gunkprojectile.BP_Gunkprojectile_C" (Math|Transform|MakeTransform (Transformation|GetActorLocation) "0, 0, 0" "1,1,1") "Undefined" 0 (* (Variables|Default|GetDirection) (* _index (/ (Variables|Default|GetMaxDistance) (Math|Conversions|ToFloat(Integer) (Variables|Default|GetNumberOfProjectiles))))) 0)))

(fn ConstructionScript)