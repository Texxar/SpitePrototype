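; BP_BossSonicWave is a boss attack projectile that sends a growing sonic wave forward to damage the player.
; On BeginPlay, a timeline lerps it forward from its spawn point along its facing while scaling it up from zero into a wide, flat shape, then destroys it.
; A Box overlap applies fixed damage to any Core_SpiteCharacter it touches, and movement uses no sweep.
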(event OnComponentBeginOverlap(Box)
  (params (OverlappedComponent :type Primitive%20Component%20Object%20Reference) (OtherActor :type Actor%20Object%20Reference) (OtherComp :type Primitive%20Component%20Object%20Reference) (OtherBodyIndex :type Integer) (bFromSweep :type Boolean) (SweepResult :type Hit%20Result%20Structure%20%28by%20ref%29))
  (bind _ascore_spite_character (Utilities|Casting|CastToCore_SpiteCharacter OtherActor))
  (Game|Damage|ApplyDamage _ascore_spite_character 2e+01 0 0))

(event EventBeginPlay
  (Variables|Default|SetStartLocation (Transformation|GetActorLocation))
  (bind _alpha (Timeline|Timeline_0 PlayFromStart)
    (:Update
      (Transformation|SetActorLocation (Math|Vector|Lerp(Vector) (Variables|Default|GetStartLocation) (+ (Variables|Default|GetStartLocation) (* (Math|Vector|GetForwardVector (Transformation|GetActorRotation)) 5e+02)) _alpha) false false)
      (Transformation|SetActorScale3D (Math|Vector|Lerp(Vector) "0, 0, 0" "5.000000,1.000000,5.000000" _alpha)))
    (:Finished
      (Actor|DestroyActor))))

(fn ConstructionScript)