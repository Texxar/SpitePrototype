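; Boss attack that moves the boss to its phase two location and then triggers an enemy spawn there.
; On BeginPlay it caches the boss transform and finds the first BP_BossPhaseTwoLocation in the level.
; A timeline drives a swept transform lerp of BossRef to that actor.
; When the timeline finishes, a short delay precedes the SpawnEnemies call on the location actor.
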(event EventBeginPlay
  (Variables|Default|SetStartTransform (Transformation|GetActorTransform (Variables|Default|GetBossRef)))
  (bind _outactors (Actor|GetAllActorsOfClass "/Game/Root_Spite/Common/Enemies/Boss/Attacks/BP_BossPhaseTwoLocation.BP_BossPhaseTwoLocation_C"))
  (bind _location (Timeline|Timeline_0 PlayFromStart)
    (:Update
      (Transformation|SetActorTransform (Variables|Default|GetBossRef) (Math|Transform|Lerp(Transform) (Variables|Default|GetStartTransform) (Transformation|GetActorTransform (Utilities|Array|Get(acopy) _outactors)) _location) true))
    (:Finished
      (Utilities|FlowControl|Delay 1.0)
      (Default|SpawnEnemies (Utilities|Array|Get(acopy) _outactors)))))

(fn ConstructionScript)