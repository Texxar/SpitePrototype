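; BP_LeechAttack is a short-lived attack actor for the Leech enemy that damages the Spite character on contact.
; On BeginPlay a timeline lerps it from its starting position to AttackLocation without sweeping, then destroys it when finished.
; An overlap on Sphere1 applies fixed damage to any Core_SpiteCharacter it touches, independently of the movement.
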(event OnComponentBeginOverlap(Sphere1)
  (params (OverlappedComponent :type Primitive%20Component%20Object%20Reference) (OtherActor :type Actor%20Object%20Reference) (OtherComp :type Primitive%20Component%20Object%20Reference) (OtherBodyIndex :type Integer) (bFromSweep :type Boolean) (SweepResult :type Hit%20Result%20Structure%20%28by%20ref%29))
  (bind _ascore_spite_character (Utilities|Casting|CastToCore_SpiteCharacter OtherActor))
  (Game|Damage|ApplyDamage _ascore_spite_character 1e+01 0 0))

(event EventBeginPlay
  (Variables|Default|SetStartLocation (Transformation|GetActorLocation))
  (bind _alpha (Timeline|Timeline_0 PlayFromStart)
    (:Update
      (Transformation|SetActorLocation (Math|Vector|Lerp(Vector) (Variables|Default|GetStartLocation) (Variables|Default|GetAttackLocation) _alpha) false false))
    (:Finished
      (Actor|DestroyActor))))

(fn ConstructionScript)