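; BP_Chest is an interactable chest that opens when a player character walks up to it and bursts into experience orbs.
; An overlap on OpenCollider by a Core_SpiteCharacter fires a DoOnce, so the chest opens only once.
; A timeline lerps the Cube1 lid between closed and tilted-open relative transforms.
; When the timeline finishes, a loop spawns a batch of BP_ExpOrb actors at the chest's location.
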(event OnComponentBeginOverlap(OpenCollider)
  (params (OverlappedComponent :type Primitive%20Component%20Object%20Reference) (OtherActor :type Actor%20Object%20Reference) (OtherComp :type Primitive%20Component%20Object%20Reference) (OtherBodyIndex :type Integer) (bFromSweep :type Boolean) (SweepResult :type Hit%20Result%20Structure%20%28by%20ref%29))
  (Utilities|Casting|CastToCore_SpiteCharacter OtherActor)
  (Utilities|FlowControl|DoOnce false
    (:Completed
      (bind _alpha (Timeline|Timeline_0 Play)
        (:Update
          (Transformation|SetRelativeTransform (Variables|Default|GetCube1) (Math|Transform|Lerp(Transform) (Math|Transform|MakeTransform "0, 0,105.000000" "0, 0, 0" "1,1.750000,0.125000") (Math|Transform|MakeTransform "-72.000000,0.000000,75.000000" "60.000000,0.000000,0.000000" "1.000000,1.750000,0.125000") _alpha) false false))
        (:Finished
          (for _index (range 0 30)
            (Game|SpawnActorfromClass "/Game/Root_Spite/Core/Framework/BP_ExpOrb.BP_ExpOrb_C" (Math|Transform|MakeTransform (Transformation|GetActorLocation) "0, 0, 0" "1,1,1") "Undefined" 0 0)))))))

(fn ConstructionScript)