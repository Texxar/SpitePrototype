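; Bloodletting platform interactable that lights up and triggers a linked object when a BP_Bloodletting actor enters its sphere.
; On BeginPlay it creates a dynamic material from the emissive circle and shares it across the circle and several other components.
; The overlap plays a timeline that ramps the material's Strength parameter to raise the glow, then sends InteractMessage to InteractObjectRef when finished.
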(event OnComponentBeginOverlap(Sphere)
  (params (OverlappedComponent :type Primitive%20Component%20Object%20Reference) (OtherActor :type Actor%20Object%20Reference) (OtherComp :type Primitive%20Component%20Object%20Reference) (OtherBodyIndex :type Integer) (bFromSweep :type Boolean) (SweepResult :type Hit%20Result%20Structure%20%28by%20ref%29))
  (Utilities|Casting|CastToBP_Bloodletting OtherActor)
  (bind _newtrack_0 (Timeline|Timeline_0 Play)
    (:Update
      (Rendering|Material|SetScalarParameterValue (Variables|Default|GetDynamicMaterial) "Strength" (Math|Float|Lerp 0.0 5.0 _newtrack_0) :!class /Script/Engine.MaterialInstanceDynamic))
    (:Finished
      (Class|BPIInteractable|Interact(Message) (Variables|Default|GetInteractObjectRef)))))

(event EventBeginPlay
  (bind _returnvalue (Rendering|Material|CreateDynamicMaterialInstance (Utilities|Array|Get(acopy) (Rendering|Material|GetMaterials (Variables|Default|GetEmissiveCircle))) "Strength" :!class /Script/Engine.KismetMaterialLibrary))
  (bind _output_get (Variables|Default|SetDynamicMaterial _returnvalue))
  (Rendering|Material|SetMaterial (Variables|Default|GetEmissiveCircle) 0 _output_get))

(fn ConstructionScript)